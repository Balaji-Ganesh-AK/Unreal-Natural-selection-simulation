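; AI spawn controller actor that populates the level with MyCh_TypeOne_BP characters on a SpawnCharacter event.
; Each spawn lands at a random navigable point in a wide radius around the actor and receives the passed game controller reference.
; A running CharacterCount, compared to half the requested count, assigns Male to early spawns and Female to the rest.
; Every character starts as Adolescent, then calculates age-based stats and applies its gender material.
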(event EventBeginPlay)

(event Collision|EventActorBeginOverlap
  (params (OtherActor :type Actor%20Object%20Reference)))

(event EventTick
  (params (DeltaSeconds :type Float%20%28single-precision%29)))

(event EventSpawnCharacter
  (params (count :type Integer) (ControllerRef :type Game%20Controller%20Actor%20Object%20Reference))
  (Utilities|FlowControl|ForLoopwithBreak 0 count
    (:LoopBody
      (bind _randomlocation (Class|NavigationSystemV1|GetRandomLocationinNavigableRadius (Transformation|GetWorldLocation (Variables|Default|GetDefaultSceneRoot)) 1e+04 0 0))
      (bind _returnvalue (Game|SpawnActorfromClass "/Game/Blueprint/Characters/MyCh_TypeOne_BP.MyCh_TypeOne_BP_C" (Math|Transform|MakeTransform _randomlocation) "Undefined" 0 0))
      (bind _result (Math|Integer|IncrementInt (Variables|Default|GetCharacterCount))
        (:%20%20
          (bind _output_get (Variables|Default|SetCharacterCount _result))
          (if (> (/ count 2) _output_get)
            (Variables|/Script/NaturalSelection.Ch_TypeOne|SetType _returnvalue "Male")
            (else
              (Variables|/Script/NaturalSelection.Ch_TypeOne|SetType _returnvalue "Female")))
          (Variables|/Script/NaturalSelection.Ch_TypeOne|SetGameControllerRef _returnvalue ControllerRef)
          (Variables|/Script/NaturalSelection.Ch_TypeOne|SetSpawnAge _returnvalue "Adolescent")
          (Class|ChTypeOne|CalculateStatsBasedonAge _returnvalue)
          (Class|ChTypeOne|ChangeMaterialBasedonGender _returnvalue))))))

(fn ConstructionScript)