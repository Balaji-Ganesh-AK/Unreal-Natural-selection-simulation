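; Actor that spawns food pickups of type Food_type1BP at random navigable points around its own location.
; The GenerateFoodFirstTime event loops over a given count, picking nav-mesh points within a large radius, increments CurrentFoodCount and passes each food a reference back to this spawner.
; BeginPlay is empty, the file's own call to the event is disconnected, and MaxFood is unused.
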(event EventBeginPlay)

(event EventGenerateFoodFirstTime
  (params (count :type Integer))
  (Utilities|FlowControl|ForLoopwithBreak 0 count
    (:LoopBody
      (bind _randomlocation (Class|NavigationSystemV1|GetRandomLocationinNavigableRadius (Transformation|GetWorldLocation (Variables|Default|GetDefaultSceneRoot)) 1e+04 0 0))
      (bind _returnvalue (Game|SpawnActorfromClass "/Game/Blueprint/Food/Food_type1BP.Food_type1BP_C" (Math|Transform|MakeTransform _randomlocation) "Undefined" 0 0))
      (bind _result (Math|Integer|IncrementInt (Variables|Default|GetCurrentFoodCount))
        (:%20%20
          (Variables|Default|SetCurrentFoodCount _result)
          (Variables|/Script/NaturalSelection.Food_type1|SetFoodControllerRef _returnvalue self))))))

(fn ConstructionScript)