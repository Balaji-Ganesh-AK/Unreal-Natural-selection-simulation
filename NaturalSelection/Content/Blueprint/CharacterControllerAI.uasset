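; AI controller for Ch_TypeOne creatures that drives food seeking and mating through the AI_BT behavior tree.
; Perception updates store seen food and set CanSeeFood when the pawn needs food; ConsumedFood clears both.
; Seeing another creature sets CanReproduce and mutual CurrentMate links if both are fertile and differ in Type.
; If either is infertile, it clears the flag but still links them; a mate-clearing branch is unconnected.
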(event OnTargetPerceptionUpdated(AIPerception)
  (params (Actor :type Actor%20Object%20Reference) (Stimulus :type AI%20Stimulus%20Structure))
  (bind _asfood_type_1 (Utilities|Casting|CastToFood_type1 Actor)
    (:then
      (bind _asch_type_one (Utilities|Casting|CastToCh_TypeOne (Pawn|GetControlledPawn)))
      (if (Variables|/Script/NaturalSelection.Ch_TypeOne|GetbNeedsFood _asch_type_one)
        (Variables|Default|SetFirstSeenFood _asfood_type_1)
        (AI|Components|Blackboard|SetValueasBool (AI|GetBlackboard 0) (Utilities|Name|MakeLiteralName "CanSeeFood") true)
        (else
          (Variables|Default|SetFirstSeenFood 0)
          (AI|Components|Blackboard|SetValueasBool (AI|GetBlackboard 0) (Utilities|Name|MakeLiteralName "CanSeeFood") false))))
    (:CastFailed
      (bind _asch_type_one_2 (Utilities|Casting|CastToCh_TypeOne Actor))
      (bind _asch_type_one_3 (Utilities|Casting|CastToCh_TypeOne (Pawn|GetControlledPawn)))
      (if (and (Variables|/Script/NaturalSelection.Ch_TypeOne|GetbCanReproduce _asch_type_one_2) (Variables|/Script/NaturalSelection.Ch_TypeOne|GetbCanReproduce _asch_type_one_3))
        (if (!= (Variables|/Script/NaturalSelection.Ch_TypeOne|GetType _asch_type_one_3) (Variables|/Script/NaturalSelection.Ch_TypeOne|GetType _asch_type_one_2))
          (Variables|/Script/NaturalSelection.Ch_TypeOne|SetCurrentMate _asch_type_one_2 _asch_type_one_3)
          (Variables|/Script/NaturalSelection.Ch_TypeOne|SetCurrentMate _asch_type_one_3 _asch_type_one_2)
          (AI|Components|Blackboard|SetValueasBool (AI|GetBlackboard 0) (Utilities|Name|MakeLiteralName "CanReproduce") true))
        (else
          (Variables|/Script/NaturalSelection.Ch_TypeOne|SetCurrentMate _asch_type_one_2 _asch_type_one_3)
          (Variables|/Script/NaturalSelection.Ch_TypeOne|SetCurrentMate _asch_type_one_3 _asch_type_one_2)
          (AI|Components|Blackboard|SetValueasBool (AI|GetBlackboard 0) (Utilities|Name|MakeLiteralName "CanReproduce") false))))))

(event EventBeginPlay
  (AI|RunBehaviorTree "/Game/Blueprint/AI/AI_BT.AI_BT"))

(event EventTick
  (params (DeltaSeconds :type Float%20%28single-precision%29)))

(fn ConstructionScript)

(fn ConsumedFood
  (bind _output_get (Variables|Default|SetFirstSeenFood 0))
  (AI|Components|Blackboard|SetValueasBool (AI|GetBlackboard 0) (Utilities|Name|MakeLiteralName "CanSeeFood") false))