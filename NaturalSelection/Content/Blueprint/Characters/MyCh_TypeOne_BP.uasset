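; Character Blueprint MyCh_TypeOne_BP that applies a configurable walk speed and shows debug readouts.
; On BeginPlay it copies its Speed variable into the character movement component's max walk speed.
; Every tick it prints the Energy value and current velocity vector to screen, with the velocity labeled as Speed.
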(event EventBeginPlay
  (Variables|/Script/Engine.CharacterMovementComponent|SetMaxWalkSpeed (Variables|Character|GetCharacterMovement) (Variables|Default|Getspeed)))

(event EventTick
  (params (DeltaSeconds :type Float%20%28single-precision%29))
  (Development|PrintString (Utilities|String|Append (Utilities|String|Append "Energy= " (Utilities|String|ToString(Float) (Variables|Default|GetEnergy))) (Utilities|String|Append "Speed= " (Utilities|String|ToString(Vector) (Transformation|GetVelocity))))))

(fn ConstructionScript)