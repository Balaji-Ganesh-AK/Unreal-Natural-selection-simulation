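; Behavior tree task that checks whether an AI-controlled Ch_TypeOne creature has a mate for reproduction.
; It reads the creature's existing CurrentMate rather than searching, and if valid writes the mate's location to TargetLocation, sets CanReproduce and succeeds.
; Without a valid mate it clears CanReproduce and fails.
; A failed controller or pawn cast leaves the task unfinished.
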(event EventReceiveExecuteAI
  (params (OwnerController :type AI%20Controller%20Object%20Reference) (ControlledPawn :type Pawn%20Object%20Reference))
  (bind _ascharacter_controller_ai (Utilities|Casting|CastToCharacterControllerAI (AI|GetAIController ControlledPawn)))
  (bind _asch_type_one (Utilities|Casting|CastToCh_TypeOne (Pawn|GetControlledPawn _ascharacter_controller_ai)))
  (Utilities|IsValid (Variables|/Script/NaturalSelection.Ch_TypeOne|GetCurrentMate _asch_type_one)
    (:Is%20Valid
      (AI|BehaviorTree|SetBlackboardValueasVector (Variables|Default|GetTargetLocation) (Transformation|GetActorLocation (Variables|/Script/NaturalSelection.Ch_TypeOne|GetCurrentMate _asch_type_one)))
      (Class|BTFunctionLibrary|SetBlackboardValueasBool (Variables|Default|GetCanReproduce) true)
      (AI|BehaviorTree|FinishExecute true))
    (:Is%20Not%20Valid
      (Class|BTFunctionLibrary|SetBlackboardValueasBool (Variables|Default|GetCanReproduce) false)
      (AI|BehaviorTree|FinishExecute false))))