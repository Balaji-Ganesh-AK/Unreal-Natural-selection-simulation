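; FindFood is a behavior tree task that passes the location of food an AI pawn has seen to its blackboard.
; On execute, it reads FirstSeenFood from the pawn's CharacterControllerAI.
; A valid food actor has its location written to a vector key and the task succeeds; otherwise it clears the CanSee key and fails.
; If the controller cast fails, the task never calls FinishExecute.
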(event EventReceiveExecuteAI
  (params (OwnerController :type AI%20Controller%20Object%20Reference) (ControlledPawn :type Pawn%20Object%20Reference))
  (bind _ascharacter_controller_ai (Utilities|Casting|CastToCharacterControllerAI (AI|GetAIController ControlledPawn)))
  (Utilities|IsValid (Variables|/Game/Blueprint/CharacterControllerAI.CharacterControllerAI_C|GetFirstSeenFood _ascharacter_controller_ai)
    (:Is%20Valid
      (AI|BehaviorTree|SetBlackboardValueasVector (Variables|Default|GetBlackBoard) (Transformation|GetActorLocation (Variables|/Game/Blueprint/CharacterControllerAI.CharacterControllerAI_C|GetFirstSeenFood _ascharacter_controller_ai)))
      (AI|BehaviorTree|FinishExecute true))
    (:Is%20Not%20Valid
      (Class|BTFunctionLibrary|SetBlackboardValueasBool (Variables|Default|GetCanSee) false)
      (AI|BehaviorTree|FinishExecute false))))